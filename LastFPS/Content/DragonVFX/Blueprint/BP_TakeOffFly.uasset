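; BP_TakeOffFly is a dragon VFX actor that repeatedly plays a desert dragon animation, presumably a take-off into flight, with timed effects.
; From BeginPlay, a delay chain starts the non-looping animation, activates the dragon effect, then two ice-breath noise effects, and later deactivates only the dragon effect.
; The custom Again event calls itself after a final delay, restarting the sequence indefinitely without Tick.
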(event Custom|again
  (Components|Animation|PlayAnimation (Variables|Default|GetSK_DesertDragon) 0 false)
  (Utilities|FlowControl|Delay 0.2)
  (Components|Activation|SetActive (Variables|Default|GetNS_Dragon) true true)
  (Utilities|FlowControl|Delay 0.7)
  (Components|Activation|SetActive (Variables|Default|GetNS_NoiseBreath_Ice) true true)
  (Components|Activation|SetActive (Variables|Default|GetNS_NoiseBreath_Ice1) true true)
  (Utilities|FlowControl|Delay 1.3)
  (Components|Activation|Deactivate (Variables|Default|GetNS_Dragon))
  (Utilities|FlowControl|Delay 1.0)
  (CallFunction|Again))

(event EventBeginPlay
  (Components|Animation|PlayAnimation (Variables|Default|GetSK_DesertDragon) 0 false)
  (Utilities|FlowControl|Delay 0.2)
  (Components|Activation|SetActive (Variables|Default|GetNS_Dragon) true true)
  (Utilities|FlowControl|Delay 0.7)
  (Components|Activation|SetActive (Variables|Default|GetNS_NoiseBreath_Ice) true true)
  (Components|Activation|SetActive (Variables|Default|GetNS_NoiseBreath_Ice1) true true)
  (Utilities|FlowControl|Delay 1.3)
  (Components|Activation|Deactivate (Variables|Default|GetNS_Dragon))
  (Utilities|FlowControl|Delay 1.0)
  (CallFunction|Again))

(event Collision|EventActorBeginOverlap
  (params (OtherActor :type Actor%20Object%20Reference)))

(event EventTick
  (params (DeltaSeconds :type Float%20%28single-precision%29)))

(fn ConstructionScript)