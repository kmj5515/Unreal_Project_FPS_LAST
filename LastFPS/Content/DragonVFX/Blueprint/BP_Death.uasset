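; BP_Death is a looping death VFX showcase for a desert dragon skeletal mesh.
; It plays the animation, then uses timed delays to stage three Niagara effects: dragon, falling dust and death.
; The death effect starts alongside a timeline that drives the materials' Dissolve parameter.
; A delay fed by the timeline then calls a custom event that resets the dissolve and replays the sequence.
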(event Custom|again
  (bind _ns_death (Variables|Default|GetNS_Death))
  (Rendering|Material|SetScalarParameterValueonMaterials (Variables|Default|GetSK_DesertDragon) "Dissolve" -1.0)
  (Components|Animation|PlayAnimation (Variables|Default|GetSK_DesertDragon) 0 false)
  (Components|Activation|SetActive (Variables|Default|GetNS_Dragon) true true)
  (Utilities|FlowControl|Delay 0.8)
  (Components|Activation|Deactivate (Variables|Default|GetNS_Dragon))
  (Utilities|FlowControl|Delay 0.5)
  (Components|Activation|SetActive (Variables|Default|GetNS_Dust_FallDown) true true)
  (Utilities|FlowControl|Delay 3.0)
  (Components|Activation|SetActive _ns_death true true)
  (bind _newtrack_0 (Timeline|Dissolve PlayFromStart)
    (:Update
      (Rendering|Material|SetScalarParameterValueonMaterials (Variables|Default|GetSK_DesertDragon) "Dissolve" _newtrack_0))
    (:Finished
      (Components|Activation|Deactivate _ns_death)))
  (Utilities|FlowControl|Delay 8.0)
  (CallFunction|Again))

(event EventBeginPlay
  (bind _ns_death (Variables|Default|GetNS_Death))
  (Components|Animation|PlayAnimation (Variables|Default|GetSK_DesertDragon) 0 false)
  (Components|Activation|SetActive (Variables|Default|GetNS_Dragon) true true)
  (Utilities|FlowControl|Delay 0.8)
  (Components|Activation|Deactivate (Variables|Default|GetNS_Dragon))
  (Utilities|FlowControl|Delay 0.5)
  (Components|Activation|SetActive (Variables|Default|GetNS_Dust_FallDown) true true)
  (Utilities|FlowControl|Delay 3.0)
  (Components|Activation|SetActive _ns_death true true)
  (bind _newtrack_0 (Timeline|Dissolve PlayFromStart)
    (:Update
      (Rendering|Material|SetScalarParameterValueonMaterials (Variables|Default|GetSK_DesertDragon) "Dissolve" _newtrack_0))
    (:Finished
      (Components|Activation|Deactivate _ns_death)))
  (Utilities|FlowControl|Delay 8.0)
  (CallFunction|Again))

(event Collision|EventActorBeginOverlap
  (params (OtherActor :type Actor%20Object%20Reference)))

(event EventTick
  (params (DeltaSeconds :type Float%20%28single-precision%29)))

(fn ConstructionScript)