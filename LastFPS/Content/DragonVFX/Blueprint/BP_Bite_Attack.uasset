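; BP_Bite_Attack is a VFX showcase actor that loops a desert dragon bite attack with its effect.
; From BeginPlay it plays a non-looping animation on the SKDesertDragon component, then after a short delay activates and resets the NSDragon effect.
; The effect is deactivated shortly after, and following a pause the custom Again event calls itself to repeat the cycle indefinitely.
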(event Custom|again
  (Components|Animation|PlayAnimation (Variables|Default|GetSK_DesertDragon) 0 false)
  (Utilities|FlowControl|Delay 0.2)
  (Components|Activation|SetActive (Variables|Default|GetNS_Dragon) true true)
  (Utilities|FlowControl|Delay 0.8)
  (Components|Activation|Deactivate (Variables|Default|GetNS_Dragon))
  (Utilities|FlowControl|Delay 1.5)
  (CallFunction|Again))

(event EventBeginPlay
  (Components|Animation|PlayAnimation (Variables|Default|GetSK_DesertDragon) 0 false)
  (Utilities|FlowControl|Delay 0.2)
  (Components|Activation|SetActive (Variables|Default|GetNS_Dragon) true true)
  (Utilities|FlowControl|Delay 0.8)
  (Components|Activation|Deactivate (Variables|Default|GetNS_Dragon))
  (Utilities|FlowControl|Delay 1.5)
  (CallFunction|Again))

(event Collision|EventActorBeginOverlap
  (params (OtherActor :type Actor%20Object%20Reference)))

(event EventTick
  (params (DeltaSeconds :type Float%20%28single-precision%29)))

(fn ConstructionScript)