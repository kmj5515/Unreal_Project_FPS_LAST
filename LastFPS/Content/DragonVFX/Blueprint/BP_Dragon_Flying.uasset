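; BP_Dragon_Flying is a VFX actor that plays a desert dragon skeletal animation alongside three particle effects in a repeating cycle.
; BeginPlay starts the cycle, playing the non-looping animation and activating the three NSDragon components with a reset.
; After a one-second delay it deactivates the effects and immediately calls the custom Again event to restart everything.
; A second delay node before that restart is left unconnected and never runs.
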(event Custom|again
  (bind _ns_dragon (Variables|Default|GetNS_Dragon))
  (bind _ns_dragon1 (Variables|Default|GetNS_Dragon1))
  (bind _ns_dragon2 (Variables|Default|GetNS_Dragon2))
  (Components|Animation|PlayAnimation (Variables|Default|GetSK_DesertDragon) 0 false)
  (Components|Activation|SetActive _ns_dragon true true)
  (Components|Activation|SetActive _ns_dragon1 true true)
  (Components|Activation|SetActive _ns_dragon2 true true)
  (Utilities|FlowControl|Delay 1.0)
  (Components|Activation|Deactivate _ns_dragon)
  (Components|Activation|Deactivate _ns_dragon1)
  (Components|Activation|Deactivate _ns_dragon2)
  (CallFunction|Again))

(event EventBeginPlay
  (bind _ns_dragon (Variables|Default|GetNS_Dragon))
  (bind _ns_dragon1 (Variables|Default|GetNS_Dragon1))
  (bind _ns_dragon2 (Variables|Default|GetNS_Dragon2))
  (Components|Animation|PlayAnimation (Variables|Default|GetSK_DesertDragon) 0 false)
  (Components|Activation|SetActive _ns_dragon true true)
  (Components|Activation|SetActive _ns_dragon1 true true)
  (Components|Activation|SetActive _ns_dragon2 true true)
  (Utilities|FlowControl|Delay 1.0)
  (Components|Activation|Deactivate _ns_dragon)
  (Components|Activation|Deactivate _ns_dragon1)
  (Components|Activation|Deactivate _ns_dragon2)
  (CallFunction|Again))

(event Collision|EventActorBeginOverlap
  (params (OtherActor :type Actor%20Object%20Reference)))

(event EventTick
  (params (DeltaSeconds :type Float%20%28single-precision%29)))

(fn ConstructionScript)