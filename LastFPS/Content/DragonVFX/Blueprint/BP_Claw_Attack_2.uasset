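; BP_Claw_Attack_2 is an actor that plays a desert dragon claw attack with VFX on an endless loop, apparently as an effect showcase.
; From BeginPlay, it plays a non-looping animation on the dragon skeletal mesh.
; Timed delays then reset and activate two pairs of dragon and footstep-dust effects in turn.
; After a final delay, the custom Again event restarts the sequence.
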(event Custom|again
  (Components|Animation|PlayAnimation (Variables|Default|GetSK_DesertDragon) 0 false)
  (Utilities|FlowControl|Delay 0.6)
  (Components|Activation|SetActive (Variables|Default|GetNS_Dragon1) true true)
  (Components|Activation|SetActive (Variables|Default|GetNS_Dust_FootStep_3) true true)
  (Utilities|FlowControl|Delay 1.0)
  (Components|Activation|SetActive (Variables|Default|GetNS_Dragon) true true)
  (Components|Activation|SetActive (Variables|Default|GetNS_Dust_FootStep_2) true true)
  (Utilities|FlowControl|Delay 1.0)
  (CallFunction|Again))

(event EventBeginPlay
  (Components|Animation|PlayAnimation (Variables|Default|GetSK_DesertDragon) 0 false)
  (Utilities|FlowControl|Delay 0.6)
  (Components|Activation|SetActive (Variables|Default|GetNS_Dragon1) true true)
  (Components|Activation|SetActive (Variables|Default|GetNS_Dust_FootStep_3) true true)
  (Utilities|FlowControl|Delay 1.0)
  (Components|Activation|SetActive (Variables|Default|GetNS_Dragon) true true)
  (Components|Activation|SetActive (Variables|Default|GetNS_Dust_FootStep_2) true true)
  (Utilities|FlowControl|Delay 1.0)
  (CallFunction|Again))

(event Collision|EventActorBeginOverlap
  (params (OtherActor :type Actor%20Object%20Reference)))

(event EventTick
  (params (DeltaSeconds :type Float%20%28single-precision%29)))

(fn ConstructionScript)