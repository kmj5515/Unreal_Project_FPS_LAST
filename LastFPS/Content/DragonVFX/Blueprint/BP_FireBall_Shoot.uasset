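; BP_FireBall_Shoot is a Dragon VFX actor in which a desert dragon repeatedly shoots projectiles.
; From BeginPlay, a loop plays the dragon's non-looping animation, waits briefly, then spawns the ProjectileBP class at the Arrow component's location and rotation with a reduced scale.
; The NextArrow event then calls itself after a random delay between MinDelay and MaxDelay, so firing continues indefinitely.
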(event Custom|NextArrow
  (bind _arrow (Variables|Default|GetArrow))
  (bind _returnvalue (Transformation|GetWorldTransform _arrow))
  (Components|Animation|PlayAnimation (Variables|Default|GetSK_DesertDragon) 0 false)
  (Utilities|FlowControl|Delay 0.2)
  (Game|SpawnActorfromClass (Variables|Default|GetProjectileBP) (Math|Transform|MakeTransform (.location _returnvalue) (.rotation _returnvalue) "0.100000,0.100000,0.100000") "Undefined" "SelectDefaultAtRuntime" 0 0)
  (Utilities|FlowControl|Delay (Math|Random|RandomFloatinRange (Variables|Default|GetMin_Delay) (Variables|Default|GetMax_Delay)))
  (CallFunction|NextArrow))

(event EventBeginPlay
  (bind _arrow (Variables|Default|GetArrow))
  (bind _returnvalue (Transformation|GetWorldTransform _arrow))
  (Components|Animation|PlayAnimation (Variables|Default|GetSK_DesertDragon) 0 false)
  (Utilities|FlowControl|Delay 0.2)
  (Game|SpawnActorfromClass (Variables|Default|GetProjectileBP) (Math|Transform|MakeTransform (.location _returnvalue) (.rotation _returnvalue) "0.100000,0.100000,0.100000") "Undefined" "SelectDefaultAtRuntime" 0 0)
  (Utilities|FlowControl|Delay (Math|Random|RandomFloatinRange (Variables|Default|GetMin_Delay) (Variables|Default|GetMax_Delay)))
  (CallFunction|NextArrow))

(fn ConstructionScript)