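; Lightning axe projectile Blueprint that flies via projectile movement and spawns an electric impact effect on hit.
; Construction script applies exposed speed, gravity, collision box scale and a wheel mode flag for the Niagara effect; BeginPlay sets whether rotation follows velocity.
; On box hit it disables collision, spawns the impact Niagara system offset along the surface normal, deactivates its own effect and destroys itself after a delay.
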(event OnComponentHit(Box)
  (params (HitComponent :type Primitive%20Component%20Object%20Reference) (OtherActor :type Actor%20Object%20Reference) (OtherComp :type Primitive%20Component%20Object%20Reference) (NormalImpulse :type Vector :default "0, 0, 0") (Hit :type Hit%20Result%20Structure%20%28by%20ref%29))
  (bind (_bblockinghit _binitialoverlap _time _distance _location _impactpoint _normal) (Collision|BreakHitResult Hit))
  (Collision|SetCollisionEnabled (Variables|Default|GetBox) "NoCollision")
  (bind _returnvalue (Niagara|SpawnSystematLocation "/Game/__LightningThunderVFX/NS/NS_Hit_Electric_01AA.NS_Hit_Electric_01AA" (+ _location (* _normal (Variables|Default|GetHitPositionOffset)))))
  (Niagara|SetNiagaraVariable(Float) _returnvalue "_ColorHue" 0.0)
  (Components|Activation|Deactivate (Variables|Default|GetNiagara))
  (Utilities|FlowControl|Delay (Variables|Default|GetDelayDestroy))
  (Actor|DestroyActor))

(event EventBeginPlay
  (Variables|/Script/Engine.ProjectileMovementComponent|SetbRotationFollowsVelocity (Variables|Default|GetProjectileMovement) (Variables|Default|GetRotationFromVelocity)))

(event Collision|EventActorBeginOverlap
  (params (OtherActor :type Actor%20Object%20Reference)))

(event EventTick
  (params (DeltaSeconds :type Float%20%28single-precision%29)))

(fn ConstructionScript
  (bind _projectilemovement (Variables|Default|GetProjectileMovement))
  (bind _speed (Variables|Default|GetSpeed))
  (bind _box (Variables|Default|GetBox))
  (Variables|/Script/Engine.ProjectileMovementComponent|SetInitialSpeed _projectilemovement _speed)
  (Variables|/Script/Engine.ProjectileMovementComponent|SetMaxSpeed _projectilemovement _speed)
  (Components|Box|SetBoxExtent _box (* (Components|Box|GetScaledBoxExtent _box) (Variables|Default|GetCollisionSizeScale)) true)
  (Variables|/Script/Engine.ProjectileMovementComponent|SetProjectileGravityScale (Variables|Default|GetProjectileMovement) (Variables|Default|GetGravity))
  (Effects|Components|ParticleSystem|SetBoolParameter (Variables|Default|GetNiagara) "WheelMOde" (Variables|Default|GetWheelMode)))