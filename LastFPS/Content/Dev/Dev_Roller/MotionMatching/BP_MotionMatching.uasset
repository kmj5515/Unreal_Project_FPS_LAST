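; BP_MotionMatching is a development character Blueprint for testing motion matching with a modular body and weapon equipping.
; The construction script makes the hair, clothing, hand, foot and shoe meshes follow the main Mesh through leader pose.
; Pressing the 1 key calls TestEquipWeapon on the WeaponComponent.
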(event Input|KeyboardEvents|1
  (params (Key :type Key%20Structure :default "None"))
  (:Pressed
    (Class|WeaponComponent|TestEquipWeapon (Variables|Default|GetWeaponComponent))))

(fn ConstructionScript
  (Components|SkinnedMesh|SetLeaderPoseComponent (Variables|Default|GetHair) (Variables|Character|GetMesh) false false))