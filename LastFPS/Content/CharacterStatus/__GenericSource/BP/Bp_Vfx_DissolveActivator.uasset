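; Dissolve activator actor that publishes a spherical dissolve zone's radius and location to shared VFX parameters.
; The Radious variable scales a Sphere component, whose world position marks the zone center.
; Both values are written to the material collection MPC_Vfx_Dissolve and the Niagara collection NPC_Vfx_Dissolve, so materials and particles can share one zone.
; The same update runs in the construction script and every Tick, covering editor changes and runtime movement.
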(event EventBeginPlay)

(event Collision|EventActorBeginOverlap
  (params (OtherActor :type Actor%20Object%20Reference)))

(event EventTick
  (params (DeltaSeconds :type Float%20%28single-precision%29))
  (bind _sphere (Variables|Default|GetSphere))
  (bind _radious (Variables|Default|GetRadious))
  (bind _returnvalue (Transformation|GetWorldLocation _sphere))
  (bind _returnvalue_2 (Math|Conversions|ToLinearColor(Vector) _returnvalue))
  (Transformation|SetWorldScale3D _sphere (Math|Conversions|ToVector(Float) (* _radious 0.02)))
  (Rendering|Material|SetScalarParameterValue "/Game/CharacterStatus/__GenericSource/Material/MF/MPC_Vfx_Dissolve.MPC_Vfx_Dissolve" "Radious" _radious :!class /Script/Engine.KismetMaterialLibrary)
  (Rendering|Material|SetVectorParameterValue "/Game/CharacterStatus/__GenericSource/Material/MF/MPC_Vfx_Dissolve.MPC_Vfx_Dissolve" "DissolveActivatorLocation" _returnvalue_2 :!class /Script/Engine.KismetMaterialLibrary)
  (bind _returnvalue_3 (Class|NiagaraFunctionLibrary|GetNiagaraParameterCollection "/Game/CharacterStatus/__GenericSource/NE/NPC_Vfx_Dissolve.NPC_Vfx_Dissolve"))
  (Effects|Components|ParticleSystem|SetFloatParameter _returnvalue_3 "Radious" _radious)
  (Effects|Components|ParticleSystem|SetVectorParameter _returnvalue_3 "DissolveActivatorLocationN" (Math|Conversions|ToVector(LinearColor) _returnvalue_2)))

(fn ConstructionScript
  (bind _sphere (Variables|Default|GetSphere))
  (bind _radious (Variables|Default|GetRadious))
  (bind _returnvalue (Transformation|GetWorldLocation _sphere))
  (bind _returnvalue_2 (Math|Conversions|ToLinearColor(Vector) _returnvalue))
  (Transformation|SetWorldScale3D _sphere (Math|Conversions|ToVector(Float) (* _radious 0.02)))
  (Rendering|Material|SetScalarParameterValue "/Game/CharacterStatus/__GenericSource/Material/MF/MPC_Vfx_Dissolve.MPC_Vfx_Dissolve" "Radious" _radious :!class /Script/Engine.KismetMaterialLibrary)
  (Rendering|Material|SetVectorParameterValue "/Game/CharacterStatus/__GenericSource/Material/MF/MPC_Vfx_Dissolve.MPC_Vfx_Dissolve" "DissolveActivatorLocation" _returnvalue_2 :!class /Script/Engine.KismetMaterialLibrary)
  (bind _returnvalue_3 (Class|NiagaraFunctionLibrary|GetNiagaraParameterCollection "/Game/CharacterStatus/__GenericSource/NE/NPC_Vfx_Dissolve.NPC_Vfx_Dissolve"))
  (Effects|Components|ParticleSystem|SetFloatParameter _returnvalue_3 "Radious" _radious)
  (Effects|Components|ParticleSystem|SetVectorParameter _returnvalue_3 "DissolveActivatorLocationN" (Math|Conversions|ToVector(LinearColor) _returnvalue_2)))