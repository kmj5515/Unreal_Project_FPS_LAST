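; BP_MotionMatching is a player character Blueprint with a modular body and debug key bindings.
; The construction script sets the main Mesh as leader pose for the hair, top, bottom, hand, foot and shoes meshes.
; Number keys trigger a test weapon equip on WeaponComponent and switch global time dilation between slow motion and normal speed.
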(event Input|KeyboardEvents|1
  (params (Key :type Key%20Structure :default "None"))
  (:Pressed
    (Class|WeaponComponent|TestEquipWeapon (Variables|Default|GetWeaponComponent))))

(event Input|KeyboardEvents|2
  (params (Key :type Key%20Structure :default "None"))
  (:Pressed
    (Utilities|Time|SetGlobalTimeDilation 0.1)))

(event Input|KeyboardEvents|3
  (params (Key :type Key%20Structure :default "None"))
  (:Pressed
    (Utilities|Time|SetGlobalTimeDilation 1.0)))

(fn ConstructionScript
  (Components|SkinnedMesh|SetLeaderPoseComponent (Variables|Default|GetHair) (Variables|Character|GetMesh) false false))